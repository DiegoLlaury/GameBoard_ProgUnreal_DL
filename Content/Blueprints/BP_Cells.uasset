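; Clickable grid cell actor that represents one tile of a board, identified by Row and Column.
; Clicks on either its Cube or Box component share one path that prints the row:column coordinate and passes the cell to BoardRef's OnTileClicked.
; The cell holds no other active logic, leaving the response to a click to the board.
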(event OnClicked(Box)
  (params (TouchedComponent :type Primitive%20Component%20Object%20Reference) (ButtonPressed :type Key%20Structure :default "None"))
  (Development|PrintString (Utilities|String|Append (Utilities|String|Append (Utilities|String|ToString(Integer) (Variables|Default|GetRow)) ":") (Utilities|String|ToString(Integer) (Variables|Default|GetColumn))))
  (Default|OnTileClicked (Variables|Default|GetBoardRef) self))

(event OnClicked(Cube)
  (params (TouchedComponent :type Primitive%20Component%20Object%20Reference) (ButtonPressed :type Key%20Structure :default "None"))
  (Development|PrintString (Utilities|String|Append (Utilities|String|Append (Utilities|String|ToString(Integer) (Variables|Default|GetRow)) ":") (Utilities|String|ToString(Integer) (Variables|Default|GetColumn))))
  (Default|OnTileClicked (Variables|Default|GetBoardRef) self))

(event EventBeginPlay)

(event Collision|EventActorBeginOverlap
  (params (OtherActor :type Actor%20Object%20Reference)))

(event EventTick
  (params (DeltaSeconds :type Float%20%28single-precision%29)))

(fn ConstructionScript)