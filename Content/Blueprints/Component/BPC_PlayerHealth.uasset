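; BPC_PlayerHealth is a player health component that tracks remaining hits and grants invincibility after damage.
; BeginPlay refills RemainingHits from MaxHits; TakeHit decrements it unless the player is invincible or out of hits.
; A surviving hit sets invincibility and starts a looping flash timer, though no timer callback or invincibility reset is shown.
; The final hit only prints a game-over debug string.
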(event Custom|TakeHit
  (bind _remaininghits (Variables|Default|GetRemainingHits))
  (if (not (or (Variables|Default|GetbIsInvicible) (<= (Variables|Default|GetRemainingHits) 0)))
    (Math|Integer|DecrementInt _remaininghits
      (:%20%20
        (if (<= _remaininghits 0)
          (Development|PrintString "HellOnGameOver")
          (else
            (Variables|Default|SetbIsInvicible true)
            (bind _returnvalue (Utilities|Time|SetTimerbyEvent 0 (Variables|Default|GetFlashInterval) true))
            (Variables|Default|SetFlashTimerHandle _returnvalue)))))))

(event EventBeginPlay
  (Variables|Default|SetRemainingHits (Variables|Default|GetMaxHits))
  (Variables|Default|SetbIsInvicible false))