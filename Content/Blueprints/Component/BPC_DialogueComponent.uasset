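; Dialogue component that steps through conversation lines stored in a data table and shows them on a dialogue widget.
; Rows are looked up by number converted to row name, and each row's NextRow links to the following line, with a negative value marking the end.
; NextDialogue advances and pushes character and text to the widget; at the end it resets to row zero, calls EndDialogue and still refreshes the widget.
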(event EventBeginPlay)

(event EventTick
  (params (DeltaSeconds :type Float%20%28single-precision%29)))

(fn GetCurrentDialogueRow
  (bind _returnvalue (Utilities|GetDataTableRow (Variables|Default|GetDialogueDataTable) (Utilities|String|StringToName (Utilities|String|ToString(Integer) (Variables|Default|GetCurrentRowNumber))))
    (:then
      (bind _output_get (Variables|Default|SetCurrentDialogueRow _returnvalue))
      (return _output_get))))

(fn GetDialogueLongforRow
  (return (.DialogueLong (Utilities|Struct|BreakSDialogueRowDatas (Variables|Default|GetCurrentDialogueRow)))))

(fn GetCharacterfromRow
  (return (.Character (Utilities|Struct|BreakSDialogueRowDatas (Variables|Default|GetCurrentDialogueRow)))))

(fn IsDialogueFinished
  (return (< (.NextRow (Utilities|Struct|BreakSDialogueRowDatas (Variables|Default|GetCurrentDialogueRow))) 0)))

(fn ReadNextRow
  (params (Widget :type WBP%20Dialogue%20UI%20Object%20Reference))
  (bind _isdialoguefinished (CallFunction|IsDialogueFinished))
  (if _isdialoguefinished
    (Variables|Default|SetCurrentRowNumber 0)
    (Default|EndDialogue Widget)
    (else
      (Variables|Default|SetCurrentRowNumber (.NextRow (Utilities|Struct|BreakSDialogueRowDatas (Variables|Default|GetCurrentDialogueRow)))))))

(fn NextDialogue
  (CallFunction|ReadNextRow (Variables|Default|GetWidget))
  (CallFunction|GetCurrentDialogueRow)
  (bind _dialoguelong (CallFunction|GetDialogueLongforRow))
  (bind _charactername (CallFunction|GetCharacterfromRow))
  (Default|UpdateDialogue (Variables|Default|GetWidget) _charactername _dialoguelong))