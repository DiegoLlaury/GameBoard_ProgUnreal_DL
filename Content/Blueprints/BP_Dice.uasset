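; Dice actor that rolls the player's movement points on click, or on a debug E key press.
; A timeline flickers random 1–6 values in the player's dice text, then calls RollDice.
; While DiceLaunch is unset, RollDice picks from fresh or rotten value arrays by durability, leaving the nested necrotized branch unreachable.
; It passes the result to BPPlayer, decrements clamped durability and sets DiceLaunch; the final durability checks do nothing.
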(event Custom|OnClicked_Event
  (Timeline|Timeline PlayFromStart
    (:Update
      (for _index (range 0 15)
        (Default|SetDiceText (Variables|Default|GetBP_Player) (Utilities|Text|ToText(Integer) (Math|Random|RandomIntegerinRange 1 6)))
        (Utilities|FlowControl|Delay 0.025)))
    (:Finished
      (CallFunction|RollDice))))

(event EventBeginPlay)

(event Collision|EventActorBeginOverlap
  (params (OtherActor :type Actor%20Object%20Reference)))

(event EventTick
  (params (DeltaSeconds :type Float%20%28single-precision%29)))

(event Input|KeyboardEvents|DebugKeyE
  (params (Key :type Key%20Structure :default "None") (ActionValue :type Input%20Action%20Value%20Structure))
  (:Pressed
    (Timeline|Timeline PlayFromStart
      (:Update
        (for _index (range 0 15)
          (Default|SetDiceText (Variables|Default|GetBP_Player) (Utilities|Text|ToText(Integer) (Math|Random|RandomIntegerinRange 1 6)))
          (Utilities|FlowControl|Delay 0.025)))
      (:Finished
        (CallFunction|RollDice)))))

(fn ConstructionScript)

(fn RollDice
  (if (not (Variables|Default|GetDiceLaunch))
    (if (> (Variables|Default|GetDurability) 4)
      (if (> (Variables|Default|GetDurability) 2)
        (LocalVariables|SetValue (.OutItem (Utilities|Array|Random (Variables|Default|GetValueFreshDice))))
        (else
          (LocalVariables|SetValue (.OutItem (Utilities|Array|Random (Variables|Default|GetValueNecrotizeDice))))))
      (else
        (LocalVariables|SetValue (.OutItem (Utilities|Array|Random (Variables|Default|GetValueRottenDice))))))
    (Default|SetDiceText (Variables|Default|GetBP_Player) (Utilities|Text|ToText(Integer) (LocalVariables|GetValue)))
    (Development|PrintString (Utilities|String|ToString(Text) (Utilities|String|SelectText "Dice result : " (Utilities|Text|ToText(Integer) (LocalVariables|GetValue)) false)))
    (Variables|/Game/Blueprints/BP_Pawn.BP_Pawn_C|SetMovementPoint (Variables|Default|GetBP_Player) (LocalVariables|GetValue))
    (bind _result (Math|Integer|DecrementInt (Math|Integer|Clamp(Integer) (Variables|Default|GetDurability) 0 (Variables|Default|GetMaxDurability)))
      (:%20%20
        (Variables|Default|SetDiceLaunch true)
        (if (not (== _result 0))
          (if (not (< _result 5))
            (if (< _result 3)
              _)))))))