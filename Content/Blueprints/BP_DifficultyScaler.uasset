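; BP_DifficultyScaler is an actor that scales zombie difficulty over elapsed time.
; BeginPlay caches all BP_Zombie actors and the first one's base speeds and attack cooldown.
; While active, Tick samples speed, detection and attack-rate curves, passing only the speed and attack multipliers to each zombie.
; The detection value and AIC_Zombie cast result go unused, and Stop halts scaling.
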(event Custom|Stop
  (Variables|Default|SetbIsActive false))

(event EventBeginPlay
  (bind _outactors (Actor|GetAllActorsOfClass "/Game/Blueprints/BP_Zombie.BP_Zombie_C"))
  (bind _output_get (Variables|Default|SetZombies _outactors))
  (Variables|Default|SetBasePatrolSpeed (Variables|/Game/Blueprints/BP_Zombie.BP_Zombie_C|GetPatrolSpeed (Utilities|Array|Get(acopy) _output_get)))
  (Variables|Default|SetBaseChaseSpeed (Variables|/Game/Blueprints/BP_Zombie.BP_Zombie_C|GetChaseSpeed (Utilities|Array|Get(acopy) _output_get)))
  (Variables|Default|SetBaseAttackCooldown (Variables|/Game/Blueprints/BP_Zombie.BP_Zombie_C|GetBaseAttackCooldown (Utilities|Array|Get(acopy) _output_get))))

(event Collision|EventActorBeginOverlap
  (params (OtherActor :type Actor%20Object%20Reference)))

(event EventTick
  (params (DeltaSeconds :type Float%20%28single-precision%29))
  (if (Variables|Default|GetbIsActive)
    (bind _output_get (Variables|Default|SetElapsedTime (+ DeltaSeconds (Variables|Default|GetElapsedTime))))
    (Variables|Default|SetSpeedMult (Math|Curves|GetFloatValue (Variables|Default|GetSpeedCurve) _output_get))
    (Variables|Default|SetDetectionMult (Math|Curves|GetFloatValue (Variables|Default|GetDetectionCurve) (Variables|Default|GetElapsedTime)))
    (Variables|Default|SetAttackMult (Math|Curves|GetFloatValue (Variables|Default|GetAttackRateCurve) (Variables|Default|GetElapsedTime)))
    (for _array_element (Variables|Default|GetZombies)
      (Default|SetDifficultyMultipliers _array_element (Variables|Default|GetSpeedMult) (Variables|Default|GetAttackMult))
      (Utilities|Casting|CastToAIC_Zombie (AI|GetAIController _array_element)))))

(fn ConstructionScript)