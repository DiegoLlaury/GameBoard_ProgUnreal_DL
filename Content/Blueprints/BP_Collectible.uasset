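; BP_Collectible is a spinning pickup that disappears when the third-person character touches it.
; BeginPlay stores the starting height, and Tick applies frame-rate-independent yaw rotation and sets Z to that height plus a sine offset.
; The sine uses BobFrequency without a time input, so the offset stays constant unless that variable changes.
; Sphere overlap casts to BP_ThirdPersonCharacter and destroys the actor, with no score or inventory update.
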(event OnComponentBeginOverlap(Sphere)
  (params (OverlappedComponent :type Primitive%20Component%20Object%20Reference) (OtherActor :type Actor%20Object%20Reference) (OtherComp :type Primitive%20Component%20Object%20Reference) (OtherBodyIndex :type Integer) (bFromSweep :type Boolean) (SweepResult :type Hit%20Result%20Structure%20%28by%20ref%29))
  (Utilities|Casting|CastToBP_ThirdPersonCharacter OtherActor)
  (Actor|DestroyActor))

(event EventBeginPlay
  (Variables|Default|SetStartZ (.z (Transformation|GetActorLocation))))

(event Collision|EventActorBeginOverlap
  (params (OtherActor :type Actor%20Object%20Reference)))

(event EventTick
  (params (DeltaSeconds :type Float%20%28single-precision%29))
  (bind _returnvalue (Transformation|GetActorLocation))
  (Class|Actor|AddActorWorldRotation (Math|Rotator|MakeRotator 0.0 0.0 (* (Variables|Default|GetRotateSpeed) DeltaSeconds)))
  (Transformation|SetActorLocation (Math|Vector|MakeVector (.x _returnvalue) (.y _returnvalue) (+ (Math|Trig|Sin(Radians) (* (* (Variables|Default|GetBobFrequency) (Math|Trig|GetPI)) 2.0)) (Variables|Default|GetStartZ))) false false))

(fn ConstructionScript)