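; BP_MiniGameManager runs a collectible minigame, resetting score and timer at BeginPlay and counting elapsed time while running.
; It caches the BP_DifficultyScaler, though nothing here uses it.
; Initial spawning makes a single loop pass, decrementing MaxCollectibles, then spawning if ActiveCollectibles is below that cap.
; Spawn points are random offsets around the manager projected onto the navmesh; spawned actors are never added to ActiveCollectibles here.
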(event Custom|SpawnInitialCollectibles
  (for _index (range 0 0)
    (Math|Integer|DecrementInt (Variables|Default|GetMaxCollectibles)
      (:%20%20
        (CallFunction|SpawnOneCollectibles)))))

(event Custom|SpawnOneCollectibles
  (if (not (>= (Utilities|Array|Length (Variables|Default|GetActiveCollectibles)) (Variables|Default|GetMaxCollectibles)))
    (bind _returnvalue (Game|SpawnActorfromClass (Variables|Default|GetCollectibleClass) (Math|Transform|MakeTransform (.ProjectedLocation (AI|Navigation|ProjectPointtoNavigation (+ (* (Math|Random|RandomUnitVector) (Variables|Default|GetSpawnRadius)) (Transformation|GetActorLocation)) 0 0 "0, 0, 0")) "0, 0, 0" "1.000000,1.000000,1.000000") "Undefined" "MultiplyWithRoot" 0 0))
    (Utilities|Casting|CastToBP_Collectible _returnvalue)))

(event EventBeginPlay
  (Variables|Default|SetbIsRunning true)
  (Variables|Default|SetScore 0)
  (Variables|Default|SetElapsedTime 0.0)
  (bind _returnvalue (Actor|GetActorOfClass "/Game/Blueprints/BP_DifficultyScaler.BP_DifficultyScaler_C"))
  (Variables|Default|SetDifficultyScalerRef _returnvalue)
  (CallFunction|SpawnInitialCollectibles))

(event Collision|EventActorBeginOverlap
  (params (OtherActor :type Actor%20Object%20Reference)))

(event EventTick
  (params (DeltaSeconds :type Float%20%28single-precision%29))
  (if (Variables|Default|GetbIsRunning)
    (Variables|Default|SetElapsedTime (+ (Variables|Default|GetElapsedTime) DeltaSeconds))))

(fn ConstructionScript)